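; Base Blueprint for a Power Spheres unit, handling team colors, fog-of-war widget visibility and sighting of other units.
; On map component init, it sets the mesh material from its team and colors the map icon as enemy, friend or ally relative to the local player.
; Its widget hides on entering fog of war and reappears on leaving.
; Pawn sensing reports seen units to its squad when that is an enemy squad.
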(event Custom|OnSeePawn
  (params (Pawn :type Pawn%20Object%20Reference))
  (bind _asbp_unit (Utilities|Casting|CastToBP_Unit Pawn))
  (bind _asbp_enemy_squad (Utilities|Casting|CastToBP_EnemySquad (Variables|Default|GetSquad)))
  (Default|UnitSeenbyUnit _asbp_enemy_squad _asbp_unit))

(event EventBeginPlay
  (EventDispatchers|BindEventtoOnSeePawn (Variables|Default|GetPawnSensing) (delegate Custom|OnSeePawn)))

(event EventInitMapComponents
  (CallFunction|SetUnitColorPerTeam))

(event EventUnitLeftFOW
  (Rendering|SetVisibility (Variables|Default|GetPowerSpheresWidget) true false))

(event EventUnitEnteredFOW
  (Rendering|SetVisibility (Variables|Default|GetPowerSpheresWidget) false false))

(fn ConstructionScript)

(fn SetUnitColorPerTeam
  (bind _team (Variables|Default|GetTeam))
  (bind _aswbp_unit_widget (Utilities|Casting|CastToWBP_UnitWidget (UserInterface|GetUserWidgetObject (Variables|Default|GetPowerSpheresWidget))))
  (LocalVariables|SetUnitWidget _aswbp_unit_widget)
  (Rendering|Material|SetMaterial (Variables|Character|GetMesh) 0 (.Value (Utilities|Map|Find (Variables|Default|GetTeamColors) (Variables|Default|GetTeam))))
  (bind _aspsplayer_controller (Utilities|Casting|CastToPSPlayerController (Game|GetPlayerController 0)))
  (bind _returnvalue (Class|PSStaticLibrary|AreEnemyTeams (Variables|/Script/PowerSpheres.PSPlayerController|GetTeam _aspsplayer_controller) _team))
  (if (> _returnvalue 0)
    (Class|MapIconComponent|SetIconDrawColor (Variables|Default|GetMapIcon) (Variables|/Game/PowerSpheres/Blueprints/UI/WBP_UnitWidget.WBP_UnitWidget_C|GetEnemyHealthBarColor (LocalVariables|GetUnitWidget)))
    (elif (== (Variables|/Script/PowerSpheres.PSPlayerController|GetTeam _aspsplayer_controller) _team)
      (Class|MapIconComponent|SetIconDrawColor (Variables|Default|GetMapIcon) (Variables|/Game/PowerSpheres/Blueprints/UI/WBP_UnitWidget.WBP_UnitWidget_C|GetFriendHealthBarColor (LocalVariables|GetUnitWidget)))
      (else
        (Class|MapIconComponent|SetIconDrawColor (Variables|Default|GetMapIcon) (Variables|/Game/PowerSpheres/Blueprints/UI/WBP_UnitWidget.WBP_UnitWidget_C|GetAllyHealthBarColor (LocalVariables|GetUnitWidget)))))))