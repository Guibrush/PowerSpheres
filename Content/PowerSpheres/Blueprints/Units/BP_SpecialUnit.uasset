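; BP_SpecialUnit is a PowerSpheres unit Blueprint that handles team coloring and fog-of-war visibility of its overhead widget.
; When map components initialize, it applies the team's material from TeamColors to the mesh.
; It also tints the map icon with the unit widget's friend or enemy health bar color, relative to the local player's team.
; Fog-of-war enter and leave events hide and show the widget.
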(event EventInitMapComponents
  (CallFunction|SetUnitColorPerTeam))

(event EventUnitLeftFOW
  (Rendering|SetVisibility (Variables|Default|GetPowerSpheresWidget) true false))

(event EventUnitEnteredFOW
  (Rendering|SetVisibility (Variables|Default|GetPowerSpheresWidget) false false))

(fn ConstructionScript)

(fn SetUnitColorPerTeam
  (bind _mapicon (Variables|Default|GetMapIcon))
  (Rendering|Material|SetMaterial (Variables|Character|GetMesh) 0 (.Value (Utilities|Map|Find (Variables|Default|GetTeamColors) (Variables|Default|GetTeam))))
  (bind _aspsplayer_controller (Utilities|Casting|CastToPSPlayerController (Game|GetPlayerController 0)))
  (bind _aswbp_unit_widget (Utilities|Casting|CastToWBP_UnitWidget (UserInterface|GetUserWidgetObject (Variables|Default|GetPowerSpheresWidget))))
  (if (Utilities|Enum|Equal(Enum) (Variables|/Script/PowerSpheres.PSPlayerController|GetTeam _aspsplayer_controller) (Variables|Default|GetTeam))
    (Class|MapIconComponent|SetIconDrawColor _mapicon (Variables|/Game/PowerSpheres/Blueprints/UI/WBP_UnitWidget.WBP_UnitWidget_C|GetFriendHealthBarColor _aswbp_unit_widget))
    (else
      (Class|MapIconComponent|SetIconDrawColor _mapicon (Variables|/Game/PowerSpheres/Blueprints/UI/WBP_UnitWidget.WBP_UnitWidget_C|GetEnemyHealthBarColor _aswbp_unit_widget)))))