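; Player controller Blueprint that creates the local player's game HUD and outlines squad units through custom depth rendering.
; Each tick it clears the previous outlines, then highlights the whole squad of a same-team unit under the cursor.
; It also highlights squads being selected, derived from the PSHUD's temporary unit selection.
; A squad-selected event enables custom depth on that squad's units without tracking them for clearing.
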(event Custom|OnSquadSelectedEvent
  (params (Squad :type PS%20Squad%20Object%20Reference))
  (for _array_element (Class|PSSquad|GetAllUnits Squad)
    (Rendering|SetRenderCustomDepth (Variables|/Script/Engine.Character|GetMesh _array_element) true)))

(event EventBeginPlay
  (if (Pawn|IsLocalPlayerController)
    (bind _returnvalue (UserInterface|CreateWidget (Variables|Default|GetHUDGame) self))
    (Utilities|IsValid _returnvalue
      (:Is%20Valid
        (UserInterface|Viewport|AddtoViewport _returnvalue 0)
        (EventDispatchers|AssignOnSquadSelected (delegate Custom|OnSquadSelectedEvent))))))

(event EventTick
  (params (DeltaSeconds :type Float%20%28single-precision%29))
  (Utilities|FlowControl|Sequence
    (:then_0
      (for _array_element (Variables|Default|GetUnitsOutlined)
        (bind _mesh (Variables|/Script/Engine.Character|GetMesh _array_element)
          (:then
            (Rendering|SetRenderCustomDepth _mesh false))
          (:else)))
      (Utilities|Array|Clear (Variables|Default|GetUnitsOutlined)))
    (:then_1
      (bind _aspsunit (Utilities|Casting|CastToPSUnit (Variables|Default|GetActorUnderCursor)))
      (if (== (Variables|Default|GetTeam) (Variables|/Script/PowerSpheres.PSSquad|GetTeam (Variables|/Script/PowerSpheres.PSUnit|GetSquad _aspsunit)))
        (for _array_element_2 (Class|PSSquad|GetAllUnits (Variables|/Script/PowerSpheres.PSUnit|GetSquad _aspsunit))
          (bind _mesh_2 (Variables|/Script/Engine.Character|GetMesh _array_element_2)
            (:then
              (Rendering|SetRenderCustomDepth _mesh_2 true)
              (Utilities|Array|AddUnique (Variables|Default|GetUnitsOutlined) _array_element_2))
            (:else)))))
    (:then_2
      (bind _squads (CallFunction|GetSquadsBeingSelected))
      (for _array_element_3 _squads
        (for _array_element_4 (Class|PSSquad|GetAllUnits _array_element_3)
          (bind _mesh_3 (Variables|/Script/Engine.Character|GetMesh _array_element_4)
            (:then
              (Rendering|SetRenderCustomDepth _mesh_3 true)
              (Utilities|Array|AddUnique (Variables|Default|GetUnitsOutlined) _array_element_4))
            (:else)))))))

(fn ConstructionScript)

(fn GetSquadsBeingSelected
  (bind _aspshud (Utilities|Casting|CastToPSHUD (HUD|GetHUD)))
  (bind _returnvalue (Class|PSHUD|GetTempSelectedUnits _aspshud))
  (for _array_element _returnvalue
    (Utilities|Array|AddUnique (LocalVariables|GetTempSquads) (Variables|/Script/PowerSpheres.PSUnit|GetSquad _array_element)))
  (return (LocalVariables|GetTempSquads)))