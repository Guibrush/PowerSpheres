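; Lobby player controller that shows the lobby menu and a live list of players with their teams.
; On BeginPlay, the local controller creates the menu, shows the cursor and starts a looping one-second timer that polls the GameState PlayerArray.
; A PlayerState-to-widget map drives adding entries, refreshing changed teams and removing departed players in the menu.
; EndPlay clears all local widgets so the match can create its own.
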(event Custom|AddPlayerInfo
  (params (PlayerState :type Player%20State%20Object%20Reference))
  (bind _menuwidgetobject (Variables|Default|GetMenuWidgetObject))
  ;[1 1 1] Set the widget for the new player and add it to the list
  (bind _returnvalue (UserInterface|CreateWidget (Variables|Default|GetPlayerInfoWidget) self))
  (bind _aswbp_lobby_player_info (Utilities|Casting|CastToWBP_LobbyPlayerInfo _returnvalue))
  (Utilities|Map|Add (Variables|Default|GetPlayersInfo) PlayerState _aswbp_lobby_player_info)
  (Default|SetPlayerName _aswbp_lobby_player_info (PlayerState|GetPlayerName PlayerState))
  (bind _aspsplayer_state (Utilities|Casting|CastToPSPlayerState PlayerState))
  (Default|SetPlayerTeam _aswbp_lobby_player_info (Utilities|String|EnumtoString (Variables|/Script/PowerSpheres.PSPlayerState|GetTeam _aspsplayer_state)))
  (Variables|/Game/PowerSpheres/Blueprints/UI/WBP_LobbyPlayerInfo.WBP_LobbyPlayerInfo_C|SetIsLocal _aswbp_lobby_player_info (== (Variables|Default|GetPlayerState) PlayerState))
  (Utilities|IsValid _menuwidgetobject
    (:Is%20Valid
      (Default|AddNewPlayer _menuwidgetobject _aswbp_lobby_player_info))))

(event Custom|RemovePlayerInfo
  (params (PlayerState :type Player%20State%20Object%20Reference))
  (bind _menuwidgetobject (Variables|Default|GetMenuWidgetObject))
  (bind _playersinfo (Variables|Default|GetPlayersInfo))
  (bind (_value _returnvalue) (Utilities|Map|Find _playersinfo PlayerState))
  ;[1 1 1] Remove a widget from the list
  (if _returnvalue
    (Utilities|IsValid _menuwidgetobject
      (:Is%20Valid
        (Default|RemovePlayer _menuwidgetobject _value)
        (Utilities|Map|Remove (Variables|Default|GetPlayersInfo) PlayerState)))))

(event Custom|CheckPlayersInLobby
  ;[1 1 1] Refresh player list
  (for _array_element (Variables|/Script/Engine.GameStateBase|GetPlayerArray (Game|GetGameState))
    (if (.ReturnValue (Utilities|Map|Find (Variables|Default|GetPlayersInfo) _array_element))
      ;;[1 1 1] Refresh an already existing player
      (bind _aspsplayer_state (Utilities|Casting|CastToPSPlayerState _array_element))
      (if (not (Utilities|Enum|Equal(Enum) (Utilities|String|ToString(Text) (Class|TextBlock|GetText (Variables|/Game/PowerSpheres/Blueprints/UI/WBP_LobbyPlayerInfo.WBP_LobbyPlayerInfo_C|GetTextTeam (.Value (Utilities|Map|Find (Variables|Default|GetPlayersInfo) _array_element))))) (Utilities|String|EnumtoString (Variables|/Script/PowerSpheres.PSPlayerState|GetTeam _aspsplayer_state))))
        (Default|RefreshPlayerInfo (.Value (Utilities|Map|Find (Variables|Default|GetPlayersInfo) _array_element)) "" (Utilities|String|EnumtoString (Variables|/Script/PowerSpheres.PSPlayerState|GetTeam _aspsplayer_state))))
      (else
        ;;[1 1 1] Add new player to the list
        (CallFunction|AddPlayerInfo _array_element))))
  ;;[1 1 1] Check if we need to remove a player from the list
  (bind _keys (Utilities|Map|Keys (Variables|Default|GetPlayersInfo)))
  (for _array_element_2 _keys
    (if (not (> (Utilities|Array|FindItem (Variables|/Script/Engine.GameStateBase|GetPlayerArray (Game|GetGameState)) _array_element_2) -1))
      (CallFunction|RemovePlayerInfo _array_element_2))))

(event EventBeginPlay
  ;[1 1 1] Set the menu widget and the refresh players timer
  (if (Pawn|IsLocalPlayerController)
    (bind _returnvalue (UserInterface|CreateWidget (Variables|Default|GetMenuWidget) self))
    (bind _aswbp_lobby_menu (Utilities|Casting|CastToWBP_LobbyMenu _returnvalue))
    (bind _output_get (Variables|Default|SetMenuWidgetObject _aswbp_lobby_menu))
    (UserInterface|Viewport|AddtoViewport _output_get 0)
    (Variables|Default|SetbShowMouseCursor true)
    (Utilities|Time|SetTimerbyEvent (delegate Custom|CheckPlayersInLobby) 1.0 true)))

(event EventEndPlay
  (params (EndPlayReason :type EEndPlayReason%20Enum :default "Destroyed"))
  ;[1 1 1] Destroy all the widgets to let the normal game create its own
  (if (Pawn|IsLocalPlayerController)
    (Viewport|RemoveAllWidgets)))

(fn ConstructionScript)