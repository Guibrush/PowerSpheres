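; BP_PowerSphereCrate is a crate that can be opened once, when a unit of the local player's team is nearby.
; TryToOpen runs a zero-length multi-sphere trace on the Visibility channel at the crate's location, within UnitsInRangeToOpenRadius.
; It compares each hit PSUnit's Team to that of player controller 0; a match sets IsOpened and returns true.
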(fn ConstructionScript)

(fn TrytoOpen
  (bind _returnvalue (Transformation|GetActorLocation))
  (if (Variables|Default|GetIsOpened)
    (return false)
    (else
      (bind _aspsplayer_controller (Utilities|Casting|CastToPSPlayerController (Game|GetPlayerController 0))
        (:then
          (Variables|Default|SetPSPlayerController _aspsplayer_controller)
          (bind _outhits (Collision|MultiSphereTraceByChannel _returnvalue _returnvalue (Variables|Default|GetUnitsInRangeToOpenRadius) "TraceTypeQuery1" false 0 "None"))
          (for _array_element _outhits
            (bind _aspsunit (Utilities|Casting|CastToPSUnit (.HitActor (Collision|BreakHitResult _array_element))))
            (if (Utilities|Enum|Equal(Enum) (Variables|/Script/PowerSpheres.PSPlayerController|GetTeam (Variables|Default|GetPSPlayerController)) (Variables|/Script/PowerSpheres.PSUnit|GetTeam _aspsunit))
              (bind _output_get (Variables|Default|SetIsOpened true))
              (return _output_get)))
          (return false))
        (:CastFailed
          (return false))))))